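; Character Blueprint for the RobotHat that derives movement values and carries a prop mesh.
; Each tick it computes Acceleration from the change in horizontal speed, scaled as a percentage of max walk speed, and a clamped Turning yaw rate.
; PastTransform caches the previous frame's velocity in its location field, alongside yaw, for these deltas.
; The construction script sets jump hold time and attaches PropMesh to the prop_rSocket on the mesh.
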(event EventBeginPlay
  (|CallParentFunction) ; This node is disabled and will not be called.\nDrag off pins to build functionality.
)

(event Collision|EventActorBeginOverlap
  (params (OtherActor :type Actor%20Object%20Reference))
  (|CallParentFunction OtherActor) ; This node is disabled and will not be called.\nDrag off pins to build functionality.
)

(event EventTick
  (params (DeltaSeconds :type Float%20%28single-precision%29))
  (bind _returnvalue (Transformation|GetVelocity))
  (bind _returnvalue_2 (Transformation|GetActorRotation))
  (|CallParentFunction DeltaSeconds)
  (Utilities|FlowControl|Sequence
    (:then_0
      ;[1 1 1] Acceleration Calculation
      (Variables|Default|SetAcceleration (* (/ (/ (- (Math|Vector2D|Vector2DLength (Math|Vector2D|MakeVector2D (.x _returnvalue) (.y _returnvalue))) (Math|Vector2D|Vector2DLength (Math|Vector2D|MakeVector2D (.x (.location (Variables|Default|GetPastTransform))) (.y (.location (Variables|Default|GetPastTransform)))))) (Utilities|Time|GetWorldDeltaSeconds)) (Variables|/Script/Engine.CharacterMovementComponent|GetMaxWalkSpeed (Variables|Character|GetCharacterMovement))) 1e+02)))
    (:then_1
      ;[1 1 1] Turn Calculation
      (Variables|Default|SetTurning (Math|Float|Clamp(Float) (/ (- (.yaw _returnvalue_2) (.yaw (.rotation (Variables|Default|GetPastTransform)))) (Utilities|Time|GetWorldDeltaSeconds)) -9e+01 9e+01)))
    (:then_2
      ;[1 1 1] Get Past transform data for next tick
      (Variables|Default|SetPastTransform (Math|Transform|MakeTransform (Math|Vector|MakeVector (.x _returnvalue) (.y _returnvalue) 0.0) (Math|Rotator|MakeRotator 0.0 0.0 (.yaw _returnvalue_2)) "1,1,1")))))

(fn ConstructionScript
  (|CallParentFunction)
  (Utilities|FlowControl|Sequence
    (:then_0
      (Variables|Default|SetJumpMaxHoldTime 0.5))
    (:then_1
      (Transformation|AttachComponentToComponent (Variables|Default|GetPropMesh) (Variables|Character|GetMesh) "prop_rSocket" "KeepRelative" "KeepRelative" "KeepRelative" true))))