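; B_OurGameMode is a game mode Blueprint that respawns the player character when it is destroyed.
; On BeginPlay it casts player 0's character to B_CharacterParent, stores its class and binds to its OnDestroyed event.
; When that fires, it spawns the stored class at SpawnTransform, which this graph never sets, and has player controller 0 possess it.
; It then calls Respawn to rebind to the new character, so the cycle repeats.
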(event Custom|PlayerDestroyed
  (params (DestroyedActor :type Actor%20Object%20Reference))
  (bind _returnvalue (Game|SpawnActorfromClass (Variables|Default|GetSpawnType) (Variables|Default|GetSpawnTransform) "Undefined" 0 0))
  (Pawn|Possess (Game|GetPlayerController 0) _returnvalue)
  (CallFunction|Respawn))

(event Custom|Respawn
  (bind _asb_character_parent (Utilities|Casting|CastToB_CharacterParent (Game|GetPlayerCharacter 0)))
  (Game|BindEventtoOnDestroyed _asb_character_parent (delegate Custom|PlayerDestroyed))
  (Variables|Default|SetSpawnType (Utilities|GetClass _asb_character_parent)))

(event EventBeginPlay
  (bind _asb_character_parent (Utilities|Casting|CastToB_CharacterParent (Game|GetPlayerCharacter 0)))
  (Game|BindEventtoOnDestroyed _asb_character_parent (delegate Custom|PlayerDestroyed))
  (Variables|Default|SetSpawnType (Utilities|GetClass _asb_character_parent)))

(event EventTick
  (params (DeltaSeconds :type Float%20%28single-precision%29)))

(fn ConstructionScript)