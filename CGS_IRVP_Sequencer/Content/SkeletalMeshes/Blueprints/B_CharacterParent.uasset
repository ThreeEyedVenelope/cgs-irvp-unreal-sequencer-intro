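; Base player Character Blueprint that handles look, movement and jumping, and kills the player on a fast fall.
; Movement input follows control-rotation yaw only, and the construction script zeroes jump hold time.
; Tick checks downward velocity and calls PlayerKilled past a threshold.
; PlayerKilled flags death, turns on physics for the body and prop meshes, and destroys the actor after a short delay.
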(event Custom|PlayerKilled
  ;[1 1 1] Kill on play falling
  (Variables|Default|SetIs%20Player%20Dead? true)
  (Utilities|FlowControl|Sequence
    (:then_0
      (Utilities|FlowControl|Delay 3.0)
      (Actor|DestroyActor))
    (:then_1
      (Physics|SetSimulatePhysics (Variables|Character|GetMesh) true))
    (:then_2
      (Physics|SetSimulatePhysics (Variables|Default|GetPropMesh) true))))

(event EventBeginPlay)

(event Collision|EventActorBeginOverlap
  (params (OtherActor :type Actor%20Object%20Reference)))

(event EventTick
  (params (DeltaSeconds :type Float%20%28single-precision%29))
  ;[1 1 1] Kill on play falling
  (if (<= (.z (Transformation|GetVelocity)) -1e+03)
    (CallFunction|PlayerKilled)))

(event Input|ActionEvents|InputActionJumpAction
  (params (Key :type Key%20Structure :default "None"))
  ;[1 1 1] Jumping
  (:Pressed
    (Character|Jump))
  (:Released
    (Character|StopJumping)))

(event Input|AxisEvents|InputAxisLookUp
  (params (AxisValue :type Float%20%28single-precision%29))
  ;[1 1 1] Look Controls
  (Pawn|Input|AddControllerPitchInput AxisValue))

(event Input|AxisEvents|InputAxisLookRight
  (params (AxisValue :type Float%20%28single-precision%29))
  ;[1 1 1] Look Controls
  (Pawn|Input|AddControllerYawInput AxisValue))

(event Input|AxisEvents|InputAxisMoveForward
  (params (AxisValue :type Float%20%28single-precision%29))
  ;[1 1 1] Movement Controls
  (Pawn|Input|AddMovementInput (Math|Vector|GetForwardVector (Math|Rotator|MakeRotator 0.0 0.0 (.Yaw (Math|Rotator|BreakRotator (Pawn|GetControlRotation :!class /Script/Engine.Pawn))))) AxisValue false))

(event Input|AxisEvents|InputAxisMoveRight
  (params (AxisValue :type Float%20%28single-precision%29))
  ;[1 1 1] Movement Controls
  (Pawn|Input|AddMovementInput (Math|Vector|GetRightVector (Math|Rotator|MakeRotator 0.0 0.0 (.Yaw (Math|Rotator|BreakRotator (Pawn|GetControlRotation :!class /Script/Engine.Pawn))))) AxisValue false))

(fn ConstructionScript
  (Variables|Default|SetJumpMaxHoldTime 0.0))